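; Player controller that keeps dependent game settings in sync when a parent setting changes.
; On BeginPlay it binds to the settings subsystem's value-changed event and switches on the setting's gameplay tag.
; Telemetry, Ray Tracing and Show HUD toggles copy their bool value to child settings, while a non-Custom Graphics Preset pushes its tag value to texture and shadow quality.
; Helper functions type-check values by casting before propagating.
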(event `self.ReceiveBeginPlay`
  (`parent.ReceiveBeginPlay`)
  (add `SFSettingsSubsystem.OnSettingValueChanged` (`SFFunctionLibrary.GetSettingsSubsystem`) (`|CreateDelegate` :!event `HandleSettingValueChanged`)))

(fn `EvaluateBoolValue`
  (params (SettingValue :type "SFSettingValue Object Reference"))
  (returns (bValid :type Boolean) (bOutBool :type Boolean))
  (bind _assf_bool_value (cast `SFSettingValue_Bool` SettingValue)
    (:`then`
      (return true (`SFSettingValue_Bool.Value` _assf_bool_value)))
    (:`CastFailed`
      (return false false))))

(fn `HandleSettingValueChanged`
  (params (SettingTag :type "GameplayTag Structure (by ref)") (NewValue :type "SFSettingValue Object Reference"))
  (bind _returnvalue (`SFFunctionLibrary.GetSettingsSubsystem`))
  (bind _returnvalue_2 (`SFFunctionLibrary.GetSettingsSubsystem`))
  (bind _returnvalue_3 (`SFFunctionLibrary.GetSettingsSubsystem`))
  (bind _newvalue (`local.NewValue`))
  (bind _newvalue_2 (`local.NewValue`))
  (bind _newvalue_3 (`local.NewValue`))
  (bind (_bvalid _biscustom) (`self.IsGraphicsPresetOnCustom` (`local.NewValue`)))
  (`|SwitchGameplayTag` SettingTag
    (:`Settings.Entry.Telemetry`
      (if (`self.EvaluateBoolValue` _newvalue_3)
        (`SFSettingsSubsystem.SetSettingValue` _returnvalue_2 (struct :`TagName` "Settings.Entry.ShowFramerate") _newvalue_3)
        (`SFSettingsSubsystem.SetSettingValue` _returnvalue_2 (struct :`TagName` "Settings.Entry.ShowLatency") _newvalue_3)))
    (:`Settings.Entry.GraphicsPreset`
      (if (and _bvalid (not _biscustom))
        (`SFSettingsSubsystem.SetSettingValue` _returnvalue_3 (struct :`TagName` "Settings.Entry.TextureQuality") (`local.NewValue`))
        (`SFSettingsSubsystem.SetSettingValue` _returnvalue_3 (struct :`TagName` "Settings.Entry.ShadowQuality") (`local.NewValue`))))
    (:`Settings.Entry.RayTracing`
      (if (`self.EvaluateBoolValue` _newvalue_2)
        (`SFSettingsSubsystem.SetSettingValue` _returnvalue (struct :`TagName` "Settings.Entry.RayTracingGI") _newvalue_2)
        (`SFSettingsSubsystem.SetSettingValue` _returnvalue (struct :`TagName` "Settings.Entry.RayTracingShadow") _newvalue_2)))
    (:`Settings.Entry.ShowHUD`
      (if (`self.EvaluateBoolValue` _newvalue)
        (`SFSettingsSubsystem.SetSettingValue` (`SFFunctionLibrary.GetSettingsSubsystem`) (struct :`TagName` "Settings.Entry.ShowMinimap") _newvalue)))))

(fn `IsGraphicsPresetOnCustom`
  (params (GraphicsPresetValue :type "SFSettingValue Object Reference"))
  (returns (bValid :type Boolean) (bIsCustom :type Boolean))
  (bind _assf_tag_value (cast `SFSettingValue_Tag` GraphicsPresetValue)
    (:`then`
      (return true (== (`SFSettingValue_Tag.Value` _assf_tag_value) (struct :`TagName` "Settings.Entry.Generic.Custom"))))
    (:`CastFailed`
      (return false false))))

(fn `UserConstructionScript`)